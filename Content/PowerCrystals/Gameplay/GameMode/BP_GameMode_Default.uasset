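; Default Power Crystals game mode Blueprint that picks a team-matched spawn point for each player.
; Its ChoosePlayerStart function gathers all actors of PlayerStartClass and returns the first PCPlayerStart whose Team equals the PCPlayerController's Team.
; The chosen start is kept in a variable that is not cleared first, so a search without a match returns whatever it already holds.
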(fn `ChoosePlayerStart`
  (params (Player :type "Controller Object Reference"))
  (returns (ReturnValue :type "Actor Object Reference"))
  (locals (PlayerController :type "PCPlayerController Object Reference") (ChoosenPlayerStart :type "PCPlayerStart Object Reference"))
  (bind _aspcplayer_controller (cast `PCPlayerController` Player)
    (:`then`
      (set `local.PlayerController` _aspcplayer_controller)
      (bind _outactors (`GameplayStatics.GetAllActorsOfClass` (`self.PlayerStartClass`)))
      (for _array_element _outactors
        (bind _aspcplayer_start (cast `PCPlayerStart` _array_element))
        (if (== (`PCPlayerStart.Team` _aspcplayer_start) (`PCPlayerController.Team` (`local.PlayerController`)))
          (set `local.ChoosenPlayerStart` _aspcplayer_start)
          (break)))
      (return (`local.ChoosenPlayerStart`)))
    (:`CastFailed`
      (return null))))

(fn `UserConstructionScript`)