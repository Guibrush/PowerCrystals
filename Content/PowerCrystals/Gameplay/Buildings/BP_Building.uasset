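; Base building actor that handles visuals for selection, preview, construction and destruction.
; Building mode changes tint the mesh through a BuildingColor parameter, with Tick showing placement validity in green or red, and toggle map components and life bar.
; Non-authority instances apply team materials and set map reveal and icon color by comparing the local player's team.
; Destruction hides life bar and map presence, plays a montage and sets a short lifespan.
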(event `self.BuildingDeselected`
  (`parent.BuildingDeselected`)
  (`SceneComponent.SetHiddenInGame` (`self.SelectionCircle`) true false))

(event `self.BuildingSelected`
  (`parent.BuildingSelected`)
  (`SceneComponent.SetHiddenInGame` (`self.SelectionCircle`) false false))

(event `self.ReceiveBeginPlay`
  (bind (_value _returnvalue) (`BlueprintMapLibrary.Map_Find` (`self.TeamMaterials`) (`self.Team`)))
  (`/Engine/EditorBlueprintResources/ActorMacros.Switch Has Authority`
    (:`Remote`
      (if _returnvalue
        (`PrimitiveComponent.SetMaterial` (`self.Mesh`) 0 _value)))))

(event `self.BPNewBuildingMode`
  (params (NewIsInConstruction :type Boolean) (NewIsInPreview :type Boolean))
  (if NewIsInPreview
    (`MapIconComponent.SetIconVisible` (`self.MapIcon`) false)
    (`MapRevealerComponent.SetRevealMode` (`self.MapRevealer`) "Off")
    (`SceneComponent.SetHiddenInGame` (`self.LifeBar`) true false)
    (`MeshComponent.SetVectorParameterValueOnMaterials` (`self.Mesh`) "BuildingColor" (`KismetMathLibrary.Conv_LinearColorToVector` (struct :`G` 1.0 :`A` 1.0)))
    (elif NewIsInConstruction
      (`MeshComponent.SetVectorParameterValueOnMaterials` (`self.Mesh`) "BuildingColor" (`KismetMathLibrary.Conv_LinearColorToVector` (struct :`A` 1.0)))
      (`self.InitMapComponents`)
      (else
        (`MeshComponent.SetVectorParameterValueOnMaterials` (`self.Mesh`) "BuildingColor" (`KismetMathLibrary.Conv_LinearColorToVector` (struct :`R` 1.0 :`G` 1.0 :`B` 1.0 :`A` 1.0)))
        (`SceneComponent.SetHiddenInGame` (`self.LifeBar`) false false)
        (bind _asbp_life_bar_widget (cast `/Game/PowerCrystals/Gameplay/UI/BP_LifeBarWidget` (`WidgetComponent.GetWidget` (`self.LifeBar`))))
        (`/Game/PowerCrystals/Gameplay/UI/BP_LifeBarWidget.InitLifeBar` _asbp_life_bar_widget self)
        (`self.InitMapComponents`)))))

(event `self.ReceiveTick`
  (params (DeltaSeconds :type "Float (single-precision)"))
  (if (`self.IsInPreview`)
    (if (`self.ValidPosition`)
      (`MeshComponent.SetVectorParameterValueOnMaterials` (`self.Mesh`) "BuildingColor" (`KismetMathLibrary.Conv_LinearColorToVector` (struct :`G` 1.0 :`A` 1.0)))
      (else
        (`MeshComponent.SetVectorParameterValueOnMaterials` (`self.Mesh`) "BuildingColor" (`KismetMathLibrary.Conv_LinearColorToVector` (struct :`R` 1.0 :`A` 1.0)))))))

(event `self.BuildingDestroyed`
  (params (Killer :type "Actor Object Reference"))
  (`parent.BuildingDestroyed` Killer)
  (`self.PlayDestruction`))

(event `PlayDestruction`
  (`self.SetLifeSpan` 5.0)
  (`SceneComponent.SetHiddenInGame` (`self.LifeBar`) true false)
  (`MapRevealerComponent.SetRevealMode` (`self.MapRevealer`) "Off")
  (`MapIconComponent.SetIconVisible` (`self.MapIcon`) false)
  (`|PlayMontage` (`self.Mesh`) (`self.DestructionAnimMontage`)))

(fn `InitMapComponents`
  (if (not (`self.HasAuthority`))
    (`|ExecutionSequence`
      (:`then_0`
        (bind _aspcplayer_controller (cast `PCPlayerController` (`GameplayStatics.GetPlayerController` 0)))
        (if (!= (`PCPlayerController.Team` _aspcplayer_controller) (`self.Team`))
          (`MapRevealerComponent.SetRevealMode` (`self.MapRevealer`) "Off")
          (else
            (`MapRevealerComponent.SetRevealMode` (`self.MapRevealer`) "Permanent"))))
      (:`then_1`
        (`MapIconComponent.SetIconVisible` (`self.MapIcon`) true)
        (bind _aspcplayer_controller_2 (cast `PCPlayerController` (`GameplayStatics.GetPlayerController` 0)))
        (if (== (`PCPlayerController.Team` _aspcplayer_controller_2) (`self.Team`))
          (`MapIconComponent.SetIconDrawColor` (`self.MapIcon`) (`self.MapIconColorSelf`))
          (else
            (`MapIconComponent.SetIconDrawColor` (`self.MapIcon`) (`self.MapIconColorFriend`))))))))

(fn `UserConstructionScript`)