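; Gameplay ability that lets the player place a building for construction.
; On activation, it spawns the configured building in preview through the player controller and selects it.
; It then waits on two input events in parallel: Selection tries to start construction mode, re-arming on failure, while Action destroys the preview.
; Successful construction start or cancellation unblocks input and ends the ability.
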(event `self.K2_ActivateAbility`
  (bind _returnvalue (`PCPlayerController.SpawnBuilding` :`self` (`self.GetPlayerController`) :`BuildingBlueprint` (`self.Building`)))
  (set `self.BuildingSpawned` _returnvalue)
  (bind _buildingspawned (`self.BuildingSpawned`)
    (:`then`
      (`PCPlayerController.SelectActors` (`self.GetPlayerController`) (`|MakeArray` _buildingspawned :!type "Actor Object Reference"))
      (`AbilityTask_WaitGameplayEvent.WaitGameplayEvent` (struct :`TagName` "InputTags.Selection") null true :!label _label
        (:`then`
          (`AbilityTask_WaitGameplayEvent.WaitGameplayEvent` (struct :`TagName` "InputTags.Action") null true
            (:`EventReceived`
              (bind _buildingspawned_2 (`self.BuildingSpawned`)
                (:`then`
                  (`Actor.K2_DestroyActor` _buildingspawned_2)
                  (`self.UnblockInput`)
                  (`self.K2_EndAbility`))
                (:`else`)))))
        (:`EventReceived`
          (bind _buildingspawned_3 (`self.BuildingSpawned`)
            (:`then`
              (bind _returnvalue_2 (`PCBuilding.InitConstructionMode` _buildingspawned_3))
              (if _returnvalue_2
                (`self.UnblockInput`)
                (`self.K2_EndAbility`)
                (else
                  (goto _label))))
            (:`else`)))))
    (:`else`)))