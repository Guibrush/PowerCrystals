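; Base unit Blueprint handling presentation: selection circle, team material, health bar, map components and death.
; InitUnit applies the Team's material, initializes the LifeBar widget and binds it to health changes.
; Without authority, InitMapComponents turns off the map revealer for other teams and colors the icon as self, friend or enemy by Team and Faction.
; On death, a montage's "Death" notify destroys the capsule, blends the mesh to physics and hides the icon.
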(event `self.OnUnitSelected`
  (`SceneComponent.SetHiddenInGame` (`self.SelectionCircle`) false false))

(event `self.OnUnitDeselected`
  (`SceneComponent.SetHiddenInGame` (`self.SelectionCircle`) true false))

(event `self.InitUnit`
  (bind (_value _returnvalue) (`BlueprintMapLibrary.Map_Find` (`self.TeamMaterials`) (`self.Team`)))
  (`|ExecutionSequence`
    (:`then_0`
      (if _returnvalue
        (`PrimitiveComponent.SetMaterial` (`self.Mesh`) 0 _value)))
    (:`then_1`
      (bind _asbp_unit_widget_life_bar (cast `/Game/PowerCrystals/Gameplay/UI/BP_UnitWidget_LifeBar` (`WidgetComponent.GetWidget` (`self.LifeBar`))))
      (`/Game/PowerCrystals/Gameplay/UI/BP_UnitWidget_LifeBar.InitLifeBar` _asbp_unit_widget_life_bar self)
      (add `self.OnHealthChanged` (delegate `HealthChanged`))
      (`self.InitMapComponents`))))

(event `HealthChanged` :!signature `self.OnHealthChanged`
  (params (NewValue :type "Float (double-precision)") (Attacker :type "Actor Object Reference"))
  (`self.UpdateLifeBar` NewValue))

(event `UpdateLifeBar`
  (params (NewHealth :type "Float (double-precision)"))
  (bind _asbp_unit_widget_life_bar (cast `/Game/PowerCrystals/Gameplay/UI/BP_UnitWidget_LifeBar` (`WidgetComponent.GetWidget` (`self.LifeBar`))))
  (`/Game/PowerCrystals/Gameplay/UI/BP_UnitWidget_LifeBar.UpdateBar` _asbp_unit_widget_life_bar NewHealth))

(event `self.OnUnitDied`
  (params (Killer :type "Actor Object Reference"))
  (`parent.OnUnitDied` Killer)
  (`self.PlayDeath`))

(event `PlayDeath`
  (`SceneComponent.SetHiddenInGame` (`self.LifeBar`) true false)
  (bind _notifyname (`|PlayMontage` (`self.Mesh`) (`self.DeathAnimMontage`))
    (:`OnNotifyBegin`
      (if (== _notifyname "Death")
        (`ActorComponent.K2_DestroyComponent` (`self.CapsuleComponent`))
        (`SkeletalMeshComponent.SetPhysicsBlendWeight` (`self.Mesh`) 1.0)
        (`SkeletalMeshComponent.SetAnimationMode` (`self.Mesh`) "AnimationCustomMode")
        (`MapIconComponent.SetIconVisible` (`self.MapIcon`) false)))))

(fn `InitMapComponents`
  (if (not (`self.HasAuthority`))
    (`|ExecutionSequence`
      (:`then_0`
        (bind _aspcplayer_controller (cast `PCPlayerController` (`GameplayStatics.GetPlayerController` 0)))
        (if (!= (`PCPlayerController.Team` _aspcplayer_controller) (`self.Team`))
          (`MapRevealerComponent.SetRevealMode` (`self.MapRevealer`) "Off")))
      (:`then_1`
        (bind _aspcplayer_controller_2 (cast `PCPlayerController` (`GameplayStatics.GetPlayerController` 0)))
        (if (== (`PCPlayerController.Team` _aspcplayer_controller_2) (`self.Team`))
          (`MapIconComponent.SetIconDrawColor` (`self.MapIcon`) (`self.MapIconColorSelf`))
          (elif (== (`PCPlayerController.Faction` _aspcplayer_controller_2) (`self.Faction`))
            (`MapIconComponent.SetIconDrawColor` (`self.MapIcon`) (`self.MapIconColorFriend`))
            (else
              (`MapIconComponent.SetIconDrawColor` (`self.MapIcon`) (`self.MapIconColorEnemy`)))))))))

(fn `UserConstructionScript`)